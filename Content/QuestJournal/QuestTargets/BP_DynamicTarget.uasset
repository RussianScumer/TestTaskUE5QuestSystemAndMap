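; BP_DynamicTarget is a quest-journal target actor that moves back and forth along the world X axis.
; On BeginPlay a Timeline drives its absolute X position while keeping the current Y and Z, without sweeping.
; A FlipFlop on the Timeline's finish alternates Reverse and Play to loop the motion.
; Disconnected leftover nodes for random offset and relative X movement never run.
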(event EventBeginPlay
  (bind _returnvalue (Transformation|GetActorLocation))
  (bind (_x _y _z) (Math|Vector|BreakVector _returnvalue))
  (bind _newtrack_0 (Timeline|Timeline Play)
    (:Update
      (Transformation|SetActorLocation (Math|Vector|MakeVector _newtrack_0 _y _z) false false))
    (:Finished
      (Utilities|FlowControl|FlipFlop
        (:A
          (Timeline|Timeline Reverse))
        (:B
          (Timeline|Timeline Play))))))

(event EventTick
  (params (DeltaSeconds :type Float%20%28single-precision%29)))

(fn ConstructionScript)